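; BP_DoorBuy_Basic is a hinged door actor that swings open when its OpenDoor event is called; it contains no purchase logic.
; BeginPlay caches the hinge's closed rotation and combines it with an OpenAngle yaw to get the open rotation.
; OpenDoor plays a timeline that lerps the hinge between them, then sets IsOpen.
; Debug prints remain, and the IsOpen guard is disconnected, so nothing here blocks re-triggering.
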(event EventBeginPlay
  (bind _output_get (Variables|Default|SetClosedRotation (Variables|/Script/Engine.SceneComponent|GetRelativeRotation (Variables|Default|GetDoorHinge))))
  (Variables|Default|SetOpenRotation (Math|Rotator|CombineRotators _output_get (Math|Rotator|MakeRotator 0.0 0.0 (Variables|Default|GetOpen_Angle)))))

(event Collision|EventActorBeginOverlap
  (params (OtherActor :type Actor%20Object%20Reference)))

(event EventTick
  (params (DeltaSeconds :type Float%20%28single-precision%29)))

(event EventOpenDoor
  (Development|PrintString "HEYYEYYELDJFLKJSFDK ")
  (bind _dooranimtrack (Timeline|DoorAnimTimeline PlayFromStart)
    (:Update
      (Transformation|SetRelativeRotation (Variables|Default|GetDoorHinge) (Math|Rotator|Lerp(Rotator) (Variables|Default|GetClosedRotation) (Variables|Default|GetOpenRotation) _dooranimtrack) false false)
      (Development|PrintString (Utilities|String|ToString(Rotator) (Math|Rotator|Lerp(Rotator) (Variables|Default|GetClosedRotation) (Variables|Default|GetOpenRotation) _dooranimtrack))))
    (:Finished
      (Variables|Default|SetbIsOpen true)
      (Development|PrintString "fuuuuuuk"))))

(fn ConstructionScript)